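; Blueprint function library for an electric shock effect on a mesh, combining a glow overlay material with Niagara bolts and sparks.
; Shock starts a point-sampling system on the skeletal or static mesh, fires seeded random line traces and spawns bolts at the hits, falling back to the start point.
; The sampler receives the calling object as callback; UpdateSystem feeds mapped sample positions to bolt targets and spark start locations.
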(fn Shock
  (params (ObjRef :type Mesh%20Component%20Object%20Reference) (BoltColor :type Linear%20Color%20Structure) (FillColor :type Linear%20Color%20Structure) (OutlineColor :type Linear%20Color%20Structure) (ActorsToIgnore :type Array%20of%20Actor%20Object%20References) (Start :type Vector) (Stream :type Random%20Stream%20Structure%20%28by%20ref%29) (Radius :type Float%20%28single-precision%29) (CenterWordlSample :type Vector) (BoltLength :type Float%20%28single-precision%29) (NumberOfBolts :type Integer) (SparkSpriteSize :type Float%20%28single-precision%29) (InnerGlowOpacity :type Float%20%28single-precision%29) (OuterGlowOpacity :type Float%20%28single-precision%29))
  (bind _returnvalue (CallFunction|SamplePoints ObjRef CenterWordlSample Radius (Class|KismetMathLibrary|RandomIntegerfromStream Stream 1000) (LocalVariables|Get__WorldContext)))
  (bind _returnvalue_2 (Rendering|Material|CreateDynamicMaterialInstance ObjRef "/VertexSourcing/Material/M_Overlay.M_Overlay" "None" :!class /Script/Engine.KismetMaterialLibrary))
  (Rendering|Material|SetScalarParameterValue _returnvalue_2 "InnerGlowOpacity" InnerGlowOpacity :!class /Script/Engine.MaterialInstanceDynamic)
  (Rendering|Material|SetScalarParameterValue _returnvalue_2 "OuterGlowOpacity" OuterGlowOpacity :!class /Script/Engine.MaterialInstanceDynamic)
  (Rendering|Material|SetVectorParameterValue _returnvalue_2 "FillColor" FillColor :!class /Script/Engine.MaterialInstanceDynamic)
  (Rendering|Material|SetVectorParameterValue _returnvalue_2 "OutlineColor" OutlineColor :!class /Script/Engine.MaterialInstanceDynamic)
  (Rendering|Material|SetOverlayMaterial ObjRef _returnvalue_2 :!class /Script/Engine.MeshComponent)
  (bind _hitarray (CallFunction|RayCastWorld NumberOfBolts Start 1e+03 ActorsToIgnore Stream (LocalVariables|Get__WorldContext)))
  (for (_array_element _array_index) _hitarray
    (if (.bBlockingHit (Collision|BreakHitResult _array_element))
      (LocalVariables|SetHitLoc (.Location (Collision|BreakHitResult _array_element)))
      (else
        (LocalVariables|SetHitLoc Start)))
    (bind _outputpin (CallFunction|LightningSourcePoint (LocalVariables|GetHitLoc) (+ _array_index (Class|KismetMathLibrary|RandomIntegerfromStream Stream 1000)) BoltColor false ObjRef BoltLength (LocalVariables|Get__WorldContext)))
    (Utilities|Array|Add (LocalVariables|Getl_SystemArray) _outputpin))
  (bind _returnvalue_3 (Niagara|SpawnSystematLocation (LocalVariables|Get__WorldContext) "/VertexSourcing/Niagara/NS_Sparks.NS_Sparks" Start))
  (Effects|Components|ParticleSystem|SetFloatParameter _returnvalue_3 "User.SpriteScale" SparkSpriteSize)
  (return (LocalVariables|Getl_SystemArray) _returnvalue_3 _returnvalue))

(fn RayCastWorld
  (params (NumberOfBolts :type Integer) (Start :type Vector) (Dist :type Float%20%28double-precision%29) (ActorsToIgnore :type Array%20of%20Actor%20Object%20References) (Stream :type Random%20Stream%20Structure%20%28by%20ref%29))
  (for _index (range 0 (Math|Integer|Max(Integer) 0 (- NumberOfBolts 1)))
    (bind _outhit (Collision|LineTraceByChannel (LocalVariables|Get__WorldContext) Start (+ Start (* (Math|Random|RandomUnitVectorfromStream Stream) Dist)) "TraceTypeQuery1" false ActorsToIgnore "None"))
    (Utilities|Array|Add (LocalVariables|GetHits) _outhit))
  (return (LocalVariables|GetHits)))

(fn LightningSourcePoint
  (params (Location :type Vector) (NewRandomSeedOffset :type Integer) (BoltColor :type Linear%20Color%20Structure) (UseSkiinned :type Boolean) (Component :type Mesh%20Component%20Object%20Reference) (BoltLength :type Float%20%28single-precision%29))
  (bind _returnvalue (Niagara|SpawnSystematLocation (LocalVariables|Get__WorldContext) "/VertexSourcing/Niagara/NS_EletricBolt.NS_EletricBolt" Location "0, 0, 0" "1.000000,1.000000,1.000000" false false))
  (Niagara|SetNiagaraVariable(Float) _returnvalue "User.Length" BoltLength)
  (Class|NiagaraComponent|SetRandomSeedOffset _returnvalue NewRandomSeedOffset)
  (Effects|Components|ParticleSystem|SetColorParameter _returnvalue "User.BoltColor" BoltColor)
  (Class|NiagaraComponent|SetVariableObject _returnvalue "User.TargetObject" (LocalVariables|Get__WorldContext))
  (Components|Activation|Activate _returnvalue true)
  (Class|NiagaraComponent|SetAutoDestroy _returnvalue true)
  (return _returnvalue))

(fn SamplePoints
  (params (Object :type Mesh%20Component%20Object%20Reference) (InValue :type Vector) (Radius :type Float%20%28single-precision%29) (NewRandomSeedOffset :type Integer))
  (bind ___worldcontext (LocalVariables|Get__WorldContext))
  (bind _returnvalue (Niagara|SpawnSystematLocation ___worldcontext "/VertexSourcing/Niagara/NS_SampleLocation.NS_SampleLocation" (Transformation|GetWorldLocation Object) "0, 0, 0" "1.000000,1.000000,1.000000" false false "None" false))
  (Class|NiagaraComponent|SetRandomSeedOffset _returnvalue NewRandomSeedOffset)
  (bind _asskeletal_mesh_component (Utilities|Casting|CastToSkeletalMeshComponent Object)
    (:then
      (Class|NiagaraComponent|SetVariableBool _returnvalue "User.bSkinned" true)
      (Class|NiagaraFunctionLibrary|OverrideSystemUserVariableSkeletalMeshComponent _returnvalue "User.Skeletal Mesh" _asskeletal_mesh_component))
    (:CastFailed
      (bind _asstatic_mesh_component (Utilities|Casting|CastToStaticMeshComponent Object)
        (:then
          (bind _returnvalue_2 (Class|VertexSourcingBPLibrary|ReturnVertexCount _asstatic_mesh_component))
          (Class|NiagaraComponent|SetVariableBool _returnvalue "User.bSkinned" false)
          (Class|NiagaraFunctionLibrary|OverrideSystemUserVariableStaticMeshComponent _returnvalue "User.Static Mesh" _asstatic_mesh_component)
          (Class|NiagaraComponent|SetVariableInt _returnvalue "User.GetNumberOfVertecs" _returnvalue_2))
        (:CastFailed
          _))))
  (Class|NiagaraComponent|SetVariableObject _returnvalue "User.CallBack" ___worldcontext)
  (Niagara|SetNiagaraVariable(Float) _returnvalue "User.Radius" Radius)
  (Niagara|SetNiagaraVariable(Vector3) _returnvalue "User.Center" InValue)
  (Components|Activation|Activate _returnvalue true)
  (Components|Activation|SetAutoActivate _returnvalue true)
  (Class|NiagaraComponent|SetAutoDestroy _returnvalue true)
  (return _returnvalue))

(fn UpdateBolts
  (params (Array :type Array%20of%20Niagara%20Component%20Object%20References) (Local :type Vector) (LocalToWP :type Map%20of%20Vectors%20to%20Structs))
  (for _array_element Array
    (if (Utilities|IsValid _array_element)
      (Niagara|SetNiagaraVariable(Vector3) _array_element "User.TargetPos" (.Value (Utilities|Map|Find LocalToWP Local)))
      (else
        (Utilities|Array|RemoveItem Array _array_element)))))

(fn UpdateSparks
  (params (SparkSystem :type Niagara%20Component%20Object%20Reference) (Index :type Integer) (Vector :type Array%20of%20Vectors) (TotalSparkAmount :type Integer))
  (Utilities|IsValid SparkSystem
    (:Is%20Valid
      (if (Utilities|Array|IsValidIndex Vector Index)
        (Niagara|SetNiagaraVariable(Vector3) SparkSystem "User.StartLocation" (Utilities|Array|Get(acopy) Vector Index))
        (Class|NiagaraComponent|SetVariableInt SparkSystem "User.TotalAmountOfParticles" TotalSparkAmount)))))

(fn UpdateSystem
  (params (BoltIndex :type Integer) (SparkIndex :type Integer) (TotalSparkAmount :type Integer) (SparkSystem :type Niagara%20Component%20Object%20Reference) (BoltSystemArray :type Array%20of%20Niagara%20Component%20Object%20References) (LocalToWP :type Map%20of%20Vectors%20to%20Structs) (BooltLocalID :type Vector%20%28by%20ref%29))
  (bind ___worldcontext (LocalVariables|Get__WorldContext))
  (CallFunction|UpdateBolts BoltSystemArray BooltLocalID LocalToWP ___worldcontext)
  (bind _values (Utilities|Map|Values LocalToWP))
  (CallFunction|UpdateSparks SparkSystem SparkIndex _values TotalSparkAmount ___worldcontext))