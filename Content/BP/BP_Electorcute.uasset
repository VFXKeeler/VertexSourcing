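; BP_Electorcute plays an electrocution effect on a referenced Actor's mesh, with bolts, sparks and vertex-color marking.
; Shock rebuilds the sample-point, bolt and spark systems, sampling around the player's location, and draws a debug sphere there.
; ParticleData maps returned local positions, carried in particle Velocity, to world positions and feeds random picks to UpdateSystem.
; The first data after each shock also paints nearby vertices red after a short delay.
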(event Custom|Shock
  (bind _returnvalue (Game|GetPlayerCharacter 0))
  (bind _stream (Variables|Default|GetStream))
  (bind _actor (Variables|Default|GetActor))
  (bind _returnvalue_2 (Actor|GetComponentbyClass _actor "/Script/Engine.MeshComponent"))
  (bind _returnvalue_3 (Transformation|GetActorLocation _returnvalue))
  (Utilities|IsValid (Variables|Default|GetActor)
    (:Is%20Valid
      (Math|Random|SetRandomStreamSeed _stream 0)
      (Utilities|FlowControl|Sequence
        (:then_0
          (Utilities|IsValid (Variables|Default|GetCurrentSampleSystem)
            (:Is%20Valid
              (Components|DestroyComponent (Variables|Default|GetCurrentSampleSystem))
              (for _array_element (Variables|Default|GetSystem%20Array)
                (Utilities|IsValid _array_element
                  (:Is%20Valid
                    (Components|DestroyComponent _array_element)))))
            (:Is%20Not%20Valid
              _))
          (Rendering|Debug|DrawDebugSphere _returnvalue_3 1e+02 12 "(R=0.000000,G=0.179629,B=1.000000,A=1.000000)" 0.0)
          (Utilities|Map|Clear (Variables|Default|GetLocalPosToWP))
          ;[1 1 1] InitilizeShock
          (bind (_systemarray _sparksystem _samplepointsystem) (CallFunction|Shock _returnvalue_2 "(R=50.000000,G=42.490162,B=0.000000,A=1.000000)" "(R=10.000000,G=1.430606,B=0.000000,A=1.000000)" "(R=9.194090,G=10.000000,B=0.585730,A=1.000000)" (Utilities|Array|MakeArray _actor) (Transformation|GetWorldLocation _returnvalue_2) _stream 1e+02 _returnvalue_3 2e+02 3 3e+01 1.0 1.0))
          (Variables|Default|SetSystem%20Array _systemarray)
          (Variables|Default|SetCurrentSampleSystem _samplepointsystem)
          (Utilities|IsValid (Variables|Default|GetSpark%20System)
            (:Is%20Valid
              (Components|DestroyComponent (Variables|Default|GetSpark%20System)))
            (:Is%20Not%20Valid
              _))
          (Variables|Default|SetSpark%20System _sparksystem))
        (:then_1
          (Utilities|FlowControl|DoOnce false) ; enters at Reset
        )))))

(event Collision|EventActorBeginOverlap
  (params (OtherActor :type Actor%20Object%20Reference)))

(event EventTick
  (params (DeltaSeconds :type Float%20%28single-precision%29)))

(event EventParticleData
  (params (Data :type Array%20of%20Basic%20Particle%20Data%20Structures) (NiagaraSystem :type Niagara%20System%20Object%20Reference) (SimulationPositionOffset :type Vector%20%28by%20ref%29 :default "0, 0, 0"))
  (bind _localpostowp (Variables|Default|GetLocalPosToWP))
  (bind _actor (Variables|Default|GetActor))
  (bind _returnvalue (Actor|GetComponentbyClass _actor "/Script/Engine.MeshComponent"))
  (Utilities|Map|Clear (Variables|Default|GetLocalPosToWP))
  (bind _array_element (Utilities|Array|ForEachLoopwithBreak Data)
    (:LoopBody
      (Utilities|Map|Add (Variables|Default|GetLocalPosToWP) (.Velocity (Utilities|Struct|BreakBasicParticleData _array_element)) (.Position (Utilities|Struct|BreakBasicParticleData _array_element))))
    (:Completed
      (Utilities|FlowControl|Sequence
        (:then_0
          (Utilities|FlowControl|DoOnce false
            (:Completed
              (Utilities|FlowControl|Delay 0.05)
              (bind _keys (Utilities|Map|Keys (Variables|Default|GetLocalPosToWP)))
              (Utilities|IsValid _returnvalue
                (:Is%20Valid
                  ;[1 1 1] UpdateColor
                  (Class|VertexSourcingBPLibrary|ChangeVertexColor _returnvalue (Math|Conversions|ToColor(LinearColor) "(R=1.000000,G=0.000000,B=0.000000,A=1.000000)") _keys 1e+01))))))
        (:then_1
          ;[1 1 1] UpdateSystem
          (bind _values (Utilities|Map|Values _localpostowp))
          (bind _keys_2 (Utilities|Map|Keys _localpostowp))
          (CallFunction|UpdateSystem 0 (Math|Random|RandomIntegerinRange 0 (Utilities|Array|Length _values)) 15 (Variables|Default|GetSpark%20System) (Variables|Default|GetSystem%20Array) _localpostowp (.OutItem (Utilities|Array|Random _keys_2))))))))

(fn ConstructionScript)